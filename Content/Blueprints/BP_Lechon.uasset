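; BP_Lechon is the player-controlled actor that jumps and collects coins.
; Jump input plays a timeline that lerps the root component's X and Z relative location, with an IsJumping flag blocking re-triggers until it finishes.
; Sphere overlaps with BP_Coin increment Tostones on the IsoLechon game instance and hide the coin rather than destroy it.
; On BeginPlay it caches a level manager reference.
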(event OnComponentBeginOverlap(Sphere)
  (params (OverlappedComponent :type Primitive%20Component%20Object%20Reference) (OtherActor :type Actor%20Object%20Reference) (OtherComp :type Primitive%20Component%20Object%20Reference) (OtherBodyIndex :type Integer) (bFromSweep :type Boolean) (SweepResult :type Hit%20Result%20Structure%20%28by%20ref%29))
  (bind _asbp_coin (Utilities|Casting|CastToBP_Coin OtherActor))
  (bind _asiso_lechon_instance (Utilities|Casting|CastToIsoLechon_Instance (Game|GetGameInstance))
    (:then
      (Variables|/Game/Blueprints/GameManagement/IsoLechon_Instance.IsoLechon_Instance_C|SetTostones _asiso_lechon_instance (+ (Variables|/Game/Blueprints/GameManagement/IsoLechon_Instance.IsoLechon_Instance_C|GetTostones _asiso_lechon_instance) 1))
      (Rendering|SetActorHiddenInGame _asbp_coin true))
    (:CastFailed
      (Development|PrintString "Failed"))))

(event EventBeginPlay
  (CallFunction|Initialize))

(event Input|ActionEvents|InputActionJump
  (params (Key :type Key%20Structure :default "None"))
  (bind _defaultsceneroot (Variables|Default|GetDefaultSceneRoot))
  (:Pressed
    (Development|PrintString "Pressed jump")
    (if (not (Variables|Default|GetisJumping))
      (Variables|Default|SetisJumping true)
      (bind _newtrack_0 (Timeline|Jump%20anim PlayFromStart)
        (:Update
          (Transformation|SetRelativeLocation _defaultsceneroot (Math|Vector|MakeVector (Math|Float|Lerp 0.0 5e+01 _newtrack_0) (.y (Variables|/Script/Engine.SceneComponent|GetRelativeLocation _defaultsceneroot)) (Math|Float|Lerp 0.0 7e+01 _newtrack_0)) false false))
        (:Finished
          (Variables|Default|SetisJumping false))))))

(fn ConstructionScript)

(fn Initialize
  (bind _output (Utilities|GetLevelManager)
    (:Is%20Valid
      (Variables|Default|SetLevelManagerRef _output))
    (:Is%20Not%20Valid
      (Development|PrintString "No Level Manager" true true "(R=1.000000,G=0.000000,B=0.021000,A=1.000000)"))))