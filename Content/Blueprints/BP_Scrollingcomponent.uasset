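; Actor component that scrolls its owning actor at the level's shared speed.
; On BeginPlay it fetches and caches the level manager.
; Each Tick it offsets the owner along its local negative X by the manager's LevelSpeed times delta seconds, without sweep or a validity check on the cached reference.
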(event EventBeginPlay
  (bind (_output _returnvalue) (CallFunction|GetLevelManager))
  (if _returnvalue
    (Variables|Default|SetLevelManagerRef _output)))

(event EventTick
  (params (DeltaSeconds :type Float%20%28single-precision%29))
  (Variables|Default|SetDelta%20Seconds DeltaSeconds)
  (bind _output_get (Variables|Default|SetMovement (* (* "-1.000000, 0, 0" (Variables|/Game/Blueprints/GameManagement/BP_LevelManager.BP_LevelManager_C|GetLevelSpeed (Variables|Default|GetLevelManagerRef))) (Variables|Default|GetDelta%20Seconds))))
  (Transformation|AddActorLocalOffset (Components|GetOwner) _output_get false false))