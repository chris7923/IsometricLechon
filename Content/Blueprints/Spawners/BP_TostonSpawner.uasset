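; BP_TostonSpawner is a spawner that lays out a row of tiles along the X axis and keeps it going by recycling them.
; On BeginPlay it spawns the tiles, placing the first at its own location and each next one a TileSize beyond RearTile.
; When a spawned actor hits bounds, it is moved behind RearTile, unhidden and becomes the new rear, so tiles are reused instead of respawned.
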(event EventBeginPlay
  (for _index (range 0 (Variables|Default|GetActorsRequiredCount))
    (if (== _index 0)
      (bind _returnvalue (CallFunction|SpawnActor))
      (Variables|Default|SetRearTile _returnvalue)
      (Variables|Default|SetTileSize 2e+02)
      (Transformation|SetActorLocation (Variables|Default|GetRearTile) (Transformation|GetActorLocation) false false)
      (else
        (bind _returnvalue_2 (CallFunction|SpawnActor))
        (Transformation|SetActorLocation _returnvalue_2 (Math|Vector|MakeVector (+ (.x (Transformation|GetActorLocation (Variables|Default|GetRearTile))) (Variables|Default|GetTileSize)) (.y (Transformation|GetActorLocation (Variables|Default|GetRearTile))) (.z (Transformation|GetActorLocation (Variables|Default|GetRearTile)))) false false)
        (Variables|Default|SetRearTile _returnvalue_2)))))

(event EventSpawnActorHitBounds
  (params (OutOfBounds :type Actor%20Object%20Reference))
  (Transformation|SetActorLocation OutOfBounds (Math|Vector|MakeVector (+ (.x (Transformation|GetActorLocation (Variables|Default|GetRearTile))) (Variables|Default|GetTileSize)) (.y (Transformation|GetActorLocation (Variables|Default|GetRearTile))) (.z (Transformation|GetActorLocation (Variables|Default|GetRearTile)))) false false)
  (bind _output_get (Variables|Default|SetRearTile OutOfBounds))
  (Rendering|SetActorHiddenInGame _output_get false))

(fn ConstructionScript
  (|CallParentFunction))