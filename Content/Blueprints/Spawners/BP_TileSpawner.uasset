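; BP_TileSpawner is a spawner that lays a row of tiles along X and recycles them as they go out of bounds.
; On BeginPlay it spawns the required count, starting at its own X and Z and chaining each tile one fixed tile width past the rear one.
; When a tile hits bounds, it moves behind RearTile and becomes the new rear.
; Each placement after the first steps Y down slightly, so successive tiles never share a depth.
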(event EventBeginPlay
  (bind _returnvalue (Transformation|GetActorLocation))
  (|CallParentFunction)
  (for _index (range 0 (Variables|Default|GetActorsRequiredCount))
    (if (== _index 0)
      (bind _returnvalue_2 (CallFunction|SpawnActor))
      (Variables|Default|SetRearTile _returnvalue_2)
      (Variables|Default|SetTileSize 311.5)
      (Transformation|SetActorLocation (Variables|Default|GetRearTile) (Math|Vector|MakeVector (.x _returnvalue) (Variables|Default|GetYPosition) (.z _returnvalue)) false false)
      (else
        (bind _output_get (Variables|Default|SetYPosition (- (Variables|Default|GetYPosition) 1.0)))
        (bind _returnvalue_3 (CallFunction|SpawnActor))
        (Transformation|SetActorLocation _returnvalue_3 (Math|Vector|MakeVector (+ (.x (Transformation|GetActorLocation (Variables|Default|GetRearTile))) (Variables|Default|GetTileSize)) _output_get (.z (Transformation|GetActorLocation (Variables|Default|GetRearTile)))) false false)
        (Variables|Default|SetRearTile _returnvalue_3)))))

(event EventSpawnActorHitBounds
  (params (OutOfBounds :type Actor%20Object%20Reference))
  (bind _output_get (Variables|Default|SetYPosition (- (Variables|Default|GetYPosition) 1.0)))
  (Transformation|SetActorLocation OutOfBounds (Math|Vector|MakeVector (+ (.x (Transformation|GetActorLocation (Variables|Default|GetRearTile))) (Variables|Default|GetTileSize)) _output_get (.z (Transformation|GetActorLocation (Variables|Default|GetRearTile)))) false false)
  (Variables|Default|SetRearTile OutOfBounds))

(fn ConstructionScript
  (|CallParentFunction))