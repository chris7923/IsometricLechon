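; BP_BaseTiles is a tile actor that scrolls steadily along negative X, apparently as a base for moving tiles.
; On BeginPlay, a fast looping timer calls MoveTile, which nudges the root's X location by a fixed step, independent of frame delta, leaving Y and Z unchanged.
; A timeline named Spline that would lerp the root's X and Z between fixed endpoints is present but never runs.
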(event Custom|MoveTile
  (bind _defaultsceneroot (Variables|Default|GetDefaultSceneRoot))
  (bind _relativelocation (Variables|/Script/Engine.SceneComponent|GetRelativeLocation _defaultsceneroot))
  (bind (_x _y _z) (Math|Vector|BreakVector _relativelocation))
  (Transformation|SetWorldLocation (Variables|Default|GetDefaultSceneRoot) (Math|Vector|MakeVector (+ _x -2.0) _y _z) false false))

(event EventBeginPlay
  (Utilities|Time|SetTimerbyEvent (delegate Custom|MoveTile) 0.01 true))

(fn ConstructionScript)